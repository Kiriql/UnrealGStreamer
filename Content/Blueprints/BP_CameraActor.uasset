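; BP_CameraActor is an actor that mirrors the player's view into a render target and runs a GStreamer pipeline during play.
; On BeginPlay it creates an RGBA8 render target at the configured resolution, assigns it to its SceneCaptureComponent2D and starts the GstPipeline component.
; Each tick it snaps its location and rotation to player 0's camera manager.
; The pipeline stops on EndPlay.
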(event `self.ReceiveBeginPlay`
  (bind (_resolution_x _resolution_y) (`KismetMathLibrary.BreakVector2D` (`self.Resolution`)))
  (bind _returnvalue (`KismetRenderingLibrary.CreateRenderTarget2D` (`KismetMathLibrary.FTrunc` _resolution_x) (`KismetMathLibrary.FTrunc` _resolution_y) "RTF_RGBA8"))
  (bind _output_get (set `self.RT` _returnvalue))
  (set `SceneCaptureComponent2D.TextureTarget` _output_get (`self.SceneCaptureComponent2D`))
  (`GstPipelineComponent.StartPipeline` (`self.GstPipeline`)))

(event `self.ReceiveEndPlay`
  (params (EndPlayReason :type "EEndPlayReason Enum" :default "Destroyed"))
  (`GstPipelineComponent.StopPipeline` (`self.GstPipeline`)))

(event `self.ReceiveTick`
  (params (DeltaSeconds :type "Float (single-precision)"))
  (bind _returnvalue (`GameplayStatics.GetPlayerCameraManager` 0))
  (`self.K2_SetActorLocation` (`PlayerCameraManager.GetCameraLocation` _returnvalue))
  (`self.K2_SetActorRotation` (`PlayerCameraManager.GetCameraRotation` _returnvalue)))

(fn `UserConstructionScript`)